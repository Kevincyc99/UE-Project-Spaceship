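; Enemy spaceship that spins into place on spawn, then advances along -Z while moving sideways on Y, reversing direction when it bumps into non-player objects.
; Tick uses a random Delay as a fire throttle, spawning bullets when the player is roughly aligned on Y.
; Ramming the player deals damage and destroys it; incoming damage updates its health widget and destroys it at zero, with an explosion on destruction.
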(event Game|Damage|EventAnyDamage
  (params (Damage :type Float%20%28single-precision%29) (DamageType :type Damage%20Type%20Object%20Reference) (InstigatedBy :type Controller%20Object%20Reference) (DamageCauser :type Actor%20Object%20Reference))
  ;[1 1 1] 被击中
  (bind _output_get (Variables|Ship|SetCurrentHealth (Math|Float|Clamp(Float) (- (Variables|Ship|GetCurrentHealth) Damage) 0.0 (Variables|Ship|GetMaxHealth))))
  (CallFunction|SyncHealth)
  (if (== _output_get 0.0)
    (Actor|DestroyActor)))

(event Collision|EventHit
  (params (MyComp :type Primitive%20Component%20Object%20Reference) (Other :type Actor%20Object%20Reference) (OtherComp :type Primitive%20Component%20Object%20Reference) (bSelfMoved :type Boolean) (HitLocation :type Vector :default "0, 0, 0") (HitNormal :type Vector :default "0, 0, 0") (NormalImpulse :type Vector :default "0, 0, 0") (Hit :type Hit%20Result%20Structure%20%28by%20ref%29))
  ;[1 1 1] 碰撞判定
  (bind _asspaceship_player_bp (Utilities|Casting|CastToSpaceshipPlayer_BP Other)
    (:then
      (Game|Damage|ApplyDamage _asspaceship_player_bp 4e+01 0 0)
      (Actor|DestroyActor))
    (:CastFailed
      (Variables|Ship|SetMovementDirection (not (Variables|Ship|GetMovementDirection))))))

(event EventDestroyed
  ;[1 1 1] 敌人死亡
  (Effects|SpawnEmitteratLocation "/Game/Arts/Particles/P_Pixel_Explosion_Enemy.P_Pixel_Explosion_Enemy" (Transformation|GetActorLocation)))

(event EventTick
  (params (DeltaSeconds :type Float%20%28single-precision%29))
  (bind _returnvalue (Game|Player|GetPlayerPawn 0))
  (bind _self self)
  ;[1 1 1] 移动
  (if (not (Variables|Ship|GetIsPlayingAnimation))
    (Transformation|AddActorWorldOffset (* (Math|Vector|MakeVector 0.0 (* (Variables|Ship|GetMoveSpeed) (Math|Float|SelectFloat 1.0 -1.0 (Variables|Ship|GetMovementDirection))) -45.0) DeltaSeconds) true)
    ;[1 1 1] 发射子弹
    (Utilities|IsValid (Game|Player|GetPlayerPawn 0)
      (:Is%20Valid
        (Utilities|FlowControl|Delay (Math|Random|RandomFloatinRange 0.4 0.6))
        (Utilities|IsValid _returnvalue
          (:Is%20Valid
            (if (<= (Math|Vector|VectorLength (* (- (Transformation|GetActorLocation _returnvalue) (Transformation|GetActorLocation)) "0,1.000000, 0")) 1e+02)
              (Game|SpawnActorfromClass "/Game/Blueprints/Bullet_BP.Bullet_BP_C" (Transformation|GetActorTransform) "AdjustIfPossibleButAlwaysSpawn" _self -3e+02 _self (Utilities|Struct|MakeLinearColor 1.0 0.3 0.2 1.0) 0))))))))

(event EventBeginPlay
  ;[1 1 1] 初始
  (Variables|Ship|SetInitialYaw (.yaw (Transformation|GetActorRotation)))
  (Variables|Ship|SetInitialLocation (Transformation|GetActorLocation))
  (Variables|Ship|SetCurrentHealth (Variables|Ship|GetMaxHealth))
  (CallFunction|SyncHealth)
  ;[1 1 1] 出生动画
  (bind _movement_lerp (Timeline|SpawnAnimation Play)
    (:Update
      (Transformation|SetActorLocation (Math|Vector|Lerp(Vector) (Variables|Ship|GetInitialLocation) (+ (Variables|Ship|GetInitialLocation) "0, 0,-110.000000") _movement_lerp) false false)
      (Transformation|SetActorRotation (Math|Rotator|MakeRotator 0.0 0.0 (Math|Float|Lerp (Variables|Ship|GetInitialYaw) (+ (Variables|Ship|GetInitialYaw) 7.2e+02) _movement_lerp))))
    (:Finished
      (Variables|Ship|SetIsPlayingAnimation false))))

(fn ConstructionScript)

(fn SyncHealth
  (bind _asenemy_status_wb (Utilities|Casting|CastToEnemyStatus_WB (UserInterface|GetWidget (Variables|Default|GetWidget))))
  (Default|SetHealth _asenemy_status_wb (Math|Float|Truncate (Variables|Ship|GetCurrentHealth)) (Math|Float|Truncate (Variables|Ship|GetMaxHealth))))