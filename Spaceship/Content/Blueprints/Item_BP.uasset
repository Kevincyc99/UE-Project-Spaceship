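; Pickup item actor that drifts through the world by Speed each tick until a SpaceshipPlayer_BP overlaps it.
; Construction creates a dynamic material on the static mesh, which BeginPlay tints with the color from the Item data.
; On player overlap it broadcasts OnPickup with the item type and player, then destroys itself, leaving the effect to listeners.
; An unconnected negative ApplyDamage node never runs.
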(event EventBeginPlay
  (Rendering|Material|SetVectorParameterValue (Variables|Item|GetMaterial) "Color" (.color (Variables|Item|GetItem)) :!class /Script/Engine.MaterialInstanceDynamic))

(event Collision|EventActorBeginOverlap
  (params (OtherActor :type Actor%20Object%20Reference))
  (bind _asspaceship_player_bp (Utilities|Casting|CastToSpaceshipPlayer_BP OtherActor))
  (Default|CallOnPickup (.itemtype (Variables|Item|GetItem)) _asspaceship_player_bp)
  (Actor|DestroyActor))

(event EventTick
  (params (DeltaSeconds :type Float%20%28single-precision%29))
  (Transformation|AddActorWorldOffset (* (Variables|Item|GetSpeed) DeltaSeconds)))

(fn ConstructionScript
  (bind _returnvalue (Rendering|Material|CreateDynamicMaterialInstance (Variables|Default|GetStaticMesh) 0 0 "None" :!class /Script/Engine.PrimitiveComponent))
  (Variables|Item|SetMaterial _returnvalue))