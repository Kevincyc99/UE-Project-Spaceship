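; Game controller actor for a spaceship shooter that owns the view camera, spawn points, status widget, lives and game over.
; A Tick-fed gate and random Delay spawn enemies; every destroyed enemy, including bottom-trigger and cleanup removals, drops a random item.
; Pickups add lives or heal through negative damage, and damage events update the health display.
; Player death shakes the camera via timeline, clears enemies, then respawns or shows game over.
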(event OnComponentBeginOverlap(BottomTrigger)
  (params (OverlappedComponent :type Primitive%20Component%20Object%20Reference) (OtherActor :type Actor%20Object%20Reference) (OtherComp :type Primitive%20Component%20Object%20Reference) (OtherBodyIndex :type Integer) (bFromSweep :type Boolean) (SweepResult :type Hit%20Result%20Structure%20%28by%20ref%29))
  ;[1 1 1] 底部碰撞
  (if (Utilities|Array|ContainsItem (Variables|Game|GetEnemies) OtherActor)
    (Actor|DestroyActor OtherActor)))

(event Custom|SpawnPlayer
  (bind _returnvalue (Game|GetPlayerController 0))
  ;[1 1 1] 生成玩家
  (CallFunction|SyncLife)
  (bind _returnvalue_2 (Game|SpawnActorfromClass "/Game/Blueprints/SpaceshipPlayer_BP.SpaceshipPlayer_BP_C" (Transformation|GetWorldTransform (Variables|Default|GetSpawnPointPlayer)) "AlwaysSpawn" 0 0))
  (Pawn|Possess _returnvalue _returnvalue_2)
  (Game|Player|SetViewTargetwithBlend _returnvalue self 0.0 "VTBlend_Linear" 0.0 false)
  ;[1 1 1] 玩家死亡
  (Game|BindEventtoOnDestroyed _returnvalue_2 (delegate Custom|OnPlayerKilled))
  ;[1 1 1] 伤害同步
  (CallFunction|SyncHealth _returnvalue_2)
  (EventDispatchers|BindEventtoOnTakeAnyDamage _returnvalue_2 (delegate Custom|OnPlayerDamaged)))

(event Custom|SpawnEnemy
  (bind _spawnpointenemy (Variables|Default|GetSpawnPointEnemy))
  (bind _returnvalue (Transformation|GetWorldTransform _spawnpointenemy))
  ;[1 1 1] 生成敌人
  (bind _returnvalue_2 (Game|SpawnActorfromClass "/Game/Blueprints/SpaceshipEnemy_BP.SpaceshipEnemy_BP_C" (Math|Transform|MakeTransform (Math|Vector|MakeVector (.x (.location _returnvalue)) (+ (.y (.location _returnvalue)) (Math|Random|RandomFloatinRange -1.5e+02 1.5e+02)) (.z (.location _returnvalue))) (.rotation _returnvalue) (.scale _returnvalue)) "AlwaysSpawn" 0 0))
  (Utilities|Array|Add (Variables|Game|GetEnemies) _returnvalue_2)
  ;[1 1 1] 绑定死亡事件
  (Game|BindEventtoOnDestroyed _returnvalue_2 (delegate Custom|OnEnemyKilled)))

(event Custom|ProcessItemDrop
  (params (Enemy :type Actor%20Object%20Reference))
  ;[1 1 1] 掉落物品
  (bind _returnvalue (Game|SpawnActorfromClass "/Game/Blueprints/Item_BP.Item_BP_C" (Transformation|GetActorTransform Enemy) "AlwaysSpawn" 0 (Utilities|Array|Get(acopy) (Variables|Game|GetItemList) (Math|Random|RandomInteger (Utilities|Array|Length (Variables|Game|GetItemList)))) 0))
  (EventDispatchers|BindEventtoOnPickup _returnvalue (delegate Custom|OnPickupItem)))

(event Custom|OnPickupItem
  (params (ItemType :type E_Item%20Enum :default "NewEnumerator0") (Actor :type Actor%20Object%20Reference))
  ;[1 1 1] 掉落物品
  (switch Utilities|FlowControl|Switch|SwitchonE_Item ItemType
    (:NewEnumerator1
      (Game|Damage|ApplyDamage Actor -2e+01 0 0))
    (:NewEnumerator2
      (CallFunction|IncreaseLife))))

(event Custom|OnPlayerKilled
  (params (DestroyedActor :type Actor%20Object%20Reference))
  ;[1 1 1] 玩家死亡
  (Game|Player|SetViewTargetwithBlend (Game|GetPlayerController 0) self 0.0 "VTBlend_Linear" 0.0 false)
  (CallFunction|PlayCameraShake -2e+01)
  (CallFunction|StopSpawnEnemy)
  (Utilities|FlowControl|Delay 2.0)
  (bind _isgameover (CallFunction|IsGameOver))
  (if _isgameover
    (CallFunction|GameOver)
    (else
      (CallFunction|DecreaseLife)
      (CallFunction|ReSpawnPlayer))))

(event Custom|ReSpawnPlayer
  ;[1 1 1] 重新生成玩家
  (CallFunction|SpawnPlayer)
  (CallFunction|StartSpawnEnemy))

(event Custom|PlayCameraShake
  (params (Intensity :type Float%20%28single-precision%29))
  ;[1 1 1] 相机震动
  (bind _movement_lerp (Timeline|CameraShake PlayFromStart)
    (:Update
      (Transformation|SetRelativeLocation (Variables|Default|GetCamera) (* _movement_lerp Intensity) false false))))

(event Custom|OnPlayerDamaged
  (params (DamagedActor :type Actor%20Object%20Reference) (Damage :type Float%20%28single-precision%29) (DamageType :type Damage%20Type%20Object%20Reference) (InstigatedBy :type Controller%20Object%20Reference) (DamageCauser :type Actor%20Object%20Reference))
  ;[1 1 1] 伤害同步
  (CallFunction|SyncHealth DamagedActor))

(event Custom|StopSpawnEnemy
  (bind _enemiesdelete (Variables|Game|GetEnemiesDelete))
  ;[1 1 1] 敌人生成规则
  (for _array_element (Variables|Game|GetEnemies)
    (Utilities|Array|Add _enemiesdelete _array_element))
  (for _array_element_2 _enemiesdelete
    (Actor|DestroyActor _array_element_2))
  (Utilities|Array|Clear _enemiesdelete)
  (Utilities|FlowControl|Gate true) ; enters at Close
)

(event Custom|StartSpawnEnemy
  ;[1 1 1] 敌人生成规则
  (Utilities|FlowControl|Gate true) ; enters at Open
)

(event Custom|GameOver
  (bind _returnvalue (Game|GetPlayerController 0))
  ;[1 1 1] 游戏结束
  (bind _returnvalue_2 (UserInterface|CreateWidget "/Game/Arts/UI/WB_GameOver.WB_GameOver_C"))
  (UserInterface|Viewport|AddtoViewport _returnvalue_2 0)
  (Variables|/Script/Engine.PlayerController|SetbShowMouseCursor _returnvalue true)
  (Input|SetInputModeGameandUI _returnvalue _returnvalue_2 "LockInFullscreen" true))

(event Custom|OnEnemyKilled
  (params (DestroyedActor :type Actor%20Object%20Reference))
  ;[1 1 1] 绑定死亡事件
  (Utilities|Array|RemoveItem (Variables|Game|GetEnemies) DestroyedActor)
  (CallFunction|ProcessItemDrop DestroyedActor))

(event EventBeginPlay
  (bind _returnvalue (Game|GetPlayerController 0))
  ;[1 1 1] 游戏开始
  (CallFunction|SpawnPlayer)
  (CallFunction|StartSpawnEnemy)
  (Variables|/Script/Engine.PlayerController|SetbShowMouseCursor _returnvalue false)
  (Input|SetInputModeGameOnly _returnvalue))

(event EventTick
  (params (DeltaSeconds :type Float%20%28single-precision%29))
  ;[1 1 1] 敌人生成规则
  (Utilities|FlowControl|Gate true
    (:Exit
      (Utilities|FlowControl|Delay (Math|Random|RandomFloatinRange 2.0 4.0))
      (CallFunction|SpawnEnemy))))

(fn ConstructionScript
  (Transformation|SetRelativeLocation (Variables|Default|GetSpawnPointPlayer) (Variables|Game|GetSpawnLocationPlayer) false false)
  (Transformation|SetRelativeLocation (Variables|Default|GetSpawnPointEnemy) (Variables|Game|GetSpawnLocationEnemy) false false)
  (Transformation|SetRelativeLocation (Variables|Default|GetBottomTrigger) (Variables|Game|GetSpawnLocationTrigger) false false)
  (Transformation|SetRelativeLocation (Variables|Default|GetPlayerStatus) (Variables|Game|GetSpawnLocationPlayerStatus) false false))

(fn SyncHealth
  (params (Player :type Actor%20Object%20Reference))
  (bind _asspaceship_player_bp (Utilities|Casting|CastToSpaceshipPlayer_BP Player))
  (Default|SetHealth (.AsPlayer%20Status%20WB (Utilities|Casting|CastToPlayerStatus_WB (UserInterface|GetWidget (Variables|Default|GetPlayerStatus)))) (/ (Variables|/Game/Blueprints/SpaceshipPlayer_BP.SpaceshipPlayer_BP_C|GetCurrentHealth _asspaceship_player_bp) (Variables|/Game/Blueprints/SpaceshipPlayer_BP.SpaceshipPlayer_BP_C|GetMaxHealth _asspaceship_player_bp))))

(fn SyncLife
  (Default|SetLife (.AsPlayer%20Status%20WB (Utilities|Casting|CastToPlayerStatus_WB (UserInterface|GetWidget (Variables|Default|GetPlayerStatus)))) (Variables|Game|GetLife)))

(fn DecreaseLife
  (Math|Integer|DecrementInt (Variables|Game|GetLife)))

(fn IsGameOver
  (return (< (Variables|Game|GetLife) 2)))

(fn IncreaseLife
  (Math|Integer|IncrementInt (Variables|Game|GetLife)
    (:%20%20
      (CallFunction|SyncLife))))