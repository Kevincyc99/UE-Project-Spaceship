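; Bullet actor that travels along the world Z axis at MoveSpeed and damages actors it overlaps.
; Tick applies a frame-rate-independent offset, and an overlap with anything other than its owner applies fixed damage and destroys the bullet.
; The construction script creates a dynamic material instance on the Bullet component, which BeginPlay tints with the Color variable.
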(event EventBeginPlay
  ;[1 1 1] 设置材质颜色
  (Rendering|Material|SetVectorParameterValue (Variables|Bullet|GetMaterial) "Color2" (Variables|Bullet|GetColor) :!class /Script/Engine.MaterialInstanceDynamic))

(event Collision|EventActorBeginOverlap
  (params (OtherActor :type Actor%20Object%20Reference))
  ;[1 1 1] 重叠造成伤害
  (if (!= OtherActor (Components|GetOwner))
    (Game|Damage|ApplyDamage OtherActor 3e+01 0 0)
    (Actor|DestroyActor)))

(event EventTick
  (params (DeltaSeconds :type Float%20%28single-precision%29))
  ;[1 1 1] 子弹移动
  (Transformation|AddActorWorldOffset (Math|Vector|MakeVector 0.0 0.0 (* DeltaSeconds (Variables|Bullet|GetMoveSpeed)))))

(fn ConstructionScript
  (bind _returnvalue (Rendering|Material|CreateDynamicMaterialInstance (Variables|Default|GetBullet) 0 0 "None" :!class /Script/Engine.PrimitiveComponent))
  (Variables|Bullet|SetMaterial _returnvalue))