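; Player spaceship for a shooter that slides sideways, fires bullets and takes damage.
; A spawn timeline raises and spins the ship, then Tick enables smoothed, swept Y-axis movement whose speed also drives a yaw tilt.
; Left mouse fires a blue-tinted Bullet_BP immediately, then repeats on a looping timer until release.
; Damage reduces clamped health; at zero a short lifespan destroys the ship, triggering a pixel explosion.
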(event Custom|Fire
  (bind _self self)
  ;[1 1 1] 发射子弹
  (Game|SpawnActorfromClass "/Game/Blueprints/Bullet_BP.Bullet_BP_C" (Transformation|GetActorTransform) "AdjustIfPossibleButAlwaysSpawn" _self 5e+02 _self (Utilities|Struct|MakeLinearColor 0.2 0.3 1.0 1.0) 0))

(event EventDestroyed
  ;[1 1 1] 玩家死亡
  (Effects|SpawnEmitteratLocation "/Game/Arts/Particles/P_Pixel_Explosion.P_Pixel_Explosion" (Transformation|GetActorLocation)))

(event Game|Damage|EventAnyDamage
  (params (Damage :type Float%20%28single-precision%29) (DamageType :type Damage%20Type%20Object%20Reference) (InstigatedBy :type Controller%20Object%20Reference) (DamageCauser :type Actor%20Object%20Reference))
  ;[1 1 1] 伤害判定
  (bind _output_get (Variables|Ship|SetCurrentHealth (Math|Float|Clamp(Float) (- (Variables|Ship|GetCurrentHealth) Damage) 0.0 (Variables|Ship|GetMaxHealth))))
  (if (== _output_get 0.0)
    (Actor|SetLifeSpan 0.01)))

(event EventTick
  (params (DeltaSeconds :type Float%20%28single-precision%29))
  ;[1 1 1] 判断是否播放完动画
  (if (not (Variables|Ship|GetIsPlayingAnimation))
    ;[1 1 1] 左右移动
    (bind _output_get (Variables|Ship|SetCurrentSpeed (Math|Interpolation|FInterpTo (Variables|Ship|GetCurrentSpeed) (* DeltaSeconds (Input|AxisValues|GetMoveRight) (Variables|Ship|GetMoveSpeed)) DeltaSeconds 1e+01)))
    (Transformation|AddActorWorldOffset (Math|Vector|MakeVector 0.0 _output_get 0.0) true)
    (Transformation|SetActorRotation (Math|Rotator|MakeRotator 0.0 0.0 (+ (* (Variables|Ship|GetCurrentSpeed) -15.0) (Variables|Ship|GetInitialYaw))))))

(event EventBeginPlay
  ;[1 1 1] 初始
  (Variables|Ship|SetInitialYaw (.yaw (Transformation|GetActorRotation)))
  (Variables|Ship|SetInitialLocation (Transformation|GetActorLocation))
  (Variables|Ship|SetCurrentHealth (Variables|Ship|GetMaxHealth))
  ;[1 1 1] 出生动画
  (bind _movement_lerp (Timeline|SpawnAnimation Play)
    (:Update
      (Transformation|SetActorLocation (Math|Vector|Lerp(Vector) (Variables|Ship|GetInitialLocation) (+ (Variables|Ship|GetInitialLocation) "0, 0,110.000000") _movement_lerp) false false)
      (Transformation|SetActorRotation (Math|Rotator|MakeRotator 0.0 0.0 (Math|Float|Lerp (Variables|Ship|GetInitialYaw) (+ (Variables|Ship|GetInitialYaw) 7.2e+02) _movement_lerp))))
    (:Finished
      (Variables|Ship|SetIsPlayingAnimation false))))

(event Input|MouseEvents|LeftMouseButton
  (params (Key :type Key%20Structure :default "None"))
  (bind _self self)
  ;[1 1 1] 发射子弹
  (:Pressed
    (Utilities|Time|SetTimerbyEvent (delegate Custom|Fire) 0.3 true)
    (Game|SpawnActorfromClass "/Game/Blueprints/Bullet_BP.Bullet_BP_C" (Transformation|GetActorTransform) "AdjustIfPossibleButAlwaysSpawn" _self 5e+02 _self (Utilities|Struct|MakeLinearColor 0.2 0.3 1.0 1.0) 0))
  (:Released
    (Utilities|Time|ClearTimerbyFunctionName 0 "Fire")))

(fn ConstructionScript)